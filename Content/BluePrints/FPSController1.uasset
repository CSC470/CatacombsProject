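; First-person player character with walking, mouse look, sprint, jump, a camera-directed dash and physics object pickup.
; Sprint raises walk speed and jump height; dash launches the character, halts it after a brief delay, then re-enables shortly afterward.
; Left click toggles holding: a debug-drawn camera line trace finds a simulating component for the PhysicsHandle, whose target follows HeldObjectLocation every Tick.
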(event `InputAction|Dash`
  (params (Key :type "Key Structure"))
  ;[1 1 1] Dash
  (:`Pressed`
    (if (`self.CanDash`)
      (`self.LaunchCharacter` (* (`SceneComponent.GetForwardVector` (`self.Camera`)) 20000.0))
      (`KismetSystemLibrary.Delay` 0.05)
      (set `self.CanDash` false)
      (`MovementComponent.StopMovementImmediately` (`self.CharacterMovement`))
      (`KismetSystemLibrary.Delay` 0.1)
      (set `self.CanDash` true))))

(event `InputAction|Jump`
  (params (Key :type "Key Structure"))
  (bind _charactermovement (`self.CharacterMovement`))
  ;[1 1 1] Jump Action
  (:`Pressed`
    (`self.Jump`)
    ;[1 1 1] Sprint Jump or Regular Jump
    (if (`self.isSprinting`)
      (set `CharacterMovementComponent.JumpZVelocity` 800.0 _charactermovement)
      (else
        (set `CharacterMovementComponent.JumpZVelocity` 420.0 _charactermovement)))))

(event `InputAxis|Horizontal`
  (params (AxisValue :type "Float (single-precision)"))
  (bind (_returnvalue_roll _returnvalue_pitch _returnvalue_yaw) (`KismetMathLibrary.BreakRotator` (`self.GetControlRotation`)))
  ;[1 1 1] Keyboard Inputs For Moving Player
  (`self.AddMovementInput` (`KismetMathLibrary.GetRightVector` (`KismetMathLibrary.MakeRotator` 0.0 0.0 _returnvalue_yaw)) AxisValue))

(event `InputAxis|Vertical`
  (params (AxisValue :type "Float (single-precision)"))
  (bind (_returnvalue_roll _returnvalue_pitch _returnvalue_yaw) (`KismetMathLibrary.BreakRotator` (`self.GetControlRotation`)))
  ;[1 1 1] Keyboard Inputs For Moving Player
  (`self.AddMovementInput` (`KismetMathLibrary.GetForwardVector` (`KismetMathLibrary.MakeRotator` 0.0 0.0 _returnvalue_yaw)) AxisValue))

(event `InputAxis|MouseLookHorizontal`
  (params (AxisValue :type "Float (single-precision)"))
  ;[1 1 1] Mouse Inputs For Moving Player's Head
  (`self.AddControllerYawInput` AxisValue))

(event `InputAction|Sprint`
  (params (Key :type "Key Structure"))
  (bind _charactermovement (`self.CharacterMovement`))
  ;[1 1 1] Sprint Button
  (:`Pressed`
    (set `CharacterMovementComponent.MaxWalkSpeed` 1200.0 _charactermovement)
    (set `self.isSprinting` true))
  (:`Released`
    (set `CharacterMovementComponent.MaxWalkSpeed` 600.0 _charactermovement)
    (set `self.isSprinting` false)))

(event `InputAxis|MouseLookVertical`
  (params (AxisValue :type "Float (single-precision)"))
  ;[1 1 1] Mouse Inputs For Moving Player's Head
  (`self.AddControllerPitchInput` AxisValue))

(event `Pick Up Object`
  (bind _camera (`self.Camera`))
  (bind _returnvalue (`SceneComponent.K2_GetComponentLocation` _camera))
  ;[1 1 1] Picking Up an Object
  (bind (_outhit _returnvalue_2) (`KismetSystemLibrary.LineTraceSingle` :`Start` _returnvalue :`End` (+ (* (`SceneComponent.GetForwardVector` _camera) 300.0) _returnvalue) :`TraceChannel` "TraceTypeQuery1" :`DrawDebugType` "ForDuration"))
  (if _returnvalue_2
    (bind (_bblockinghit _binitialoverlap _time _distance _location _impactpoint _normal _impactnormal _physmat _hitactor _hitcomponent) (`GameplayStatics.BreakHitResult` _outhit))
    (if (`SceneComponent.IsSimulatingPhysics` _hitcomponent "None")
      (`PhysicsHandleComponent.GrabComponentAtLocationWithRotation` (`self.PhysicsHandle`) _hitcomponent "None" (`SceneComponent.K2_GetComponentLocation` _hitcomponent) (`KismetMathLibrary.Conv_VectorToRotator` (`KismetMathLibrary.MakeVector` 0.0)))
      (set `self.IsHoldingObject` true))))

(event `Drop Object`
  ;[1 1 1] Droping an Object
  (`PhysicsHandleComponent.ReleaseComponent` (`self.PhysicsHandle`))
  (set `self.IsHoldingObject` false))

(event `self.ReceiveTick`
  (params (DeltaSeconds :type "Float (single-precision)"))
  ;[1 1 1] Update Function
  (`PhysicsHandleComponent.SetTargetLocation` (`self.PhysicsHandle`) (`SceneComponent.K2_GetComponentLocation` (`self.HeldObjectLocation`))))

(event `Key|LeftMouseButton`
  (params (Key :type "Key Structure"))
  ;[1 1 1] Click Mouse to Pick Up Object
  (:`Pressed`
    (if (`self.IsHoldingObject`)
      (`self.Drop Object`)
      (else
        (`self.Pick Up Object`)))))

(fn `UserConstructionScript`)